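; Hero is a Paper2D flipbook character with left, right and up movement input and a jump on the Up action.
; Axis events feed world-space movement input along X and Z, and BeginPlay sets the idle flipbook.
; Animation is unfinished: Tick calls an empty UpdateAnimation, while the flying and punching flipbook events have no callers here and the velocity-based flipbook switch is disconnected.
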(event `self.ReceiveTick`
  (params (DeltaSeconds :type "Float (single-precision)"))
  ;[1 1 1] Other flip
  (`self.UpdateAnimation`))

(event `self.ReceiveBeginPlay`
  (`PaperFlipbookComponent.SetFlipbook` (`self.Sprite`) "/Game/Maps/Assets/superhero/_actions/idle.idle"))

(event `UpdateAnimation`
  ;[1 1 1] Other flip
)

(event `InputAxis|Right`
  (params (AxisValue :type "Float (single-precision)"))
  ;[1 1 1] Movement
  (`self.AddMovementInput` (1.0 0.0 0.0) AxisValue))

(event `InputAction|Up`
  (params (Key :type "Key Structure")))

(event `InputAxis|Left`
  (params (AxisValue :type "Float (single-precision)"))
  ;[1 1 1] Movement
  (`self.AddMovementInput` (-1.0 0.0 0.0) AxisValue))

(event `InputAxis|Up`
  (params (AxisValue :type "Float (single-precision)")))

(event `HandleAnimations`
  (bind _sprite (`self.Sprite`))
  (if (`self.is flying`)
    (`PaperFlipbookComponent.SetFlipbook` _sprite "/Game/Maps/Assets/superhero/_actions/flying.flying")
    (elif (`self.is punching`)
      (`PaperFlipbookComponent.SetFlipbook` _sprite null))))

(event `InputAxis|Up`
  (params (AxisValue :type "Float (single-precision)"))
  ;[1 1 1] Movement
  (`self.AddMovementInput` (0.0 0.0 1.0) AxisValue :!label _label))

(event `InputAction|Up`
  (params (Key :type "Key Structure"))
  ;[1 1 1] Movement
  (:`Pressed`
    (`self.Jump`)
    (goto _label)))

(event `Flying`
  (if true
    (`PaperFlipbookComponent.SetFlipbook` (`self.Sprite`) "/Game/Maps/Assets/superhero/_actions/flyup.flyup")))

(fn `UserConstructionScript`)